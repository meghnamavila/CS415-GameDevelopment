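; BP_Projectile is a projectile that flies along world X and destroys actors it hits, except the player and other projectiles.
; On BeginPlay it sets its speed to twice the player's ForwardSpeed, then moves by that speed each Tick using a world offset.
; The Projectile component's hit event destroys only the other actor, while a timer calls DeleteAll to remove the projectile after a few seconds.
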(event `self.ReceiveBeginPlay`
  (bind _asbp_player (cast `/Game/InfiniteMatrix/Blueprints/BP_Player` (`GameplayStatics.GetPlayerPawn` 0)))
  (set `self.Speed` (* (`/Game/InfiniteMatrix/Blueprints/BP_Player.ForwardSpeed` _asbp_player) 2.0))
  (`KismetSystemLibrary.K2_SetTimer` null "DeleteAll" 5.0))

(event `self.ReceiveActorBeginOverlap`
  (params (OtherActor :type "Actor Object Reference")))

(event `self.ReceiveTick`
  (params (DeltaSeconds :type "Float (single-precision)"))
  (`self.K2_AddActorWorldOffset` (`KismetMathLibrary.MakeVector` (* DeltaSeconds (`self.Speed`)))))

(event `self.Projectile.OnComponentHit`
  (params (HitComponent :type "PrimitiveComponent Object Reference") (OtherActor :type "Actor Object Reference") (OtherComp :type "PrimitiveComponent Object Reference") (NormalImpulse :type "Vector Structure") (Hit :type "HitResult Structure (by ref)"))
  (cast `/Game/InfiniteMatrix/Blueprints/BP_Projectile` OtherActor
    (:`CastFailed`
      (cast `/Game/InfiniteMatrix/Blueprints/BP_Player` OtherActor
        (:`CastFailed`
          (`self.K2_DestroyActor` OtherActor))))))

(fn `DeleteAll`
  (`self.K2_DestroyActor`))

(fn `UserConstructionScript`)