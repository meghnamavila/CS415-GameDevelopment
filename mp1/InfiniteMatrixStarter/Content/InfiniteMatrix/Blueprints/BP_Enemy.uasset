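; BP_Enemy is a short-lived enemy actor that reacts to overlaps on its Enemy component.
; Touching BP_Player calls CollideEnemy and shows the restart prompt if the player is dead.
; A BP_Projectile hit destroys the enemy and notifies the player pawn through ShootEnemy.
; A timer set on BeginPlay calls DeleteAll to destroy the enemy after a fixed lifetime.
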(event `self.ReceiveBeginPlay`
  (`KismetSystemLibrary.K2_SetTimer` null "DeleteAll" 10.0))

(event `self.Enemy.OnComponentBeginOverlap`
  (params (OverlappedComponent :type "PrimitiveComponent Object Reference") (OtherActor :type "Actor Object Reference") (OtherComp :type "PrimitiveComponent Object Reference") (OtherBodyIndex :type Integer) (bFromSweep :type Boolean) (SweepResult :type "HitResult Structure (by ref)"))
  (bind _asbp_player (cast `/Game/InfiniteMatrix/Blueprints/BP_Player` OtherActor)
    (:`then`
      (`/Game/InfiniteMatrix/Blueprints/BP_Player.CollideEnemy` _asbp_player)
      (if (`/Game/InfiniteMatrix/Blueprints/BP_Player.isDead` _asbp_player)
        (`/Game/InfiniteMatrix/Blueprints/BP_Player.DisplayRestart` _asbp_player)))
    (:`CastFailed`
      (cast `/Game/InfiniteMatrix/Blueprints/BP_Projectile` OtherActor)
      (`self.K2_DestroyActor`)
      (bind _asbp_player_2 (cast `/Game/InfiniteMatrix/Blueprints/BP_Player` (`GameplayStatics.GetPlayerPawn` 0)))
      (`/Game/InfiniteMatrix/Blueprints/BP_Player.ShootEnemy` _asbp_player_2))))

(fn `DeleteAll`
  (`self.K2_DestroyActor`))

(fn `UserConstructionScript`)